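; GA_Dash is a Gameplay Ability that dashes the avatar along its forward vector.
; On activation it commits, sends that vector through UpdateFacingTargetMessage and spawns a Niagara effect at the avatar's transform.
; It starts a montage and immediately applies a short constant root-motion force with gravity enabled, setting a finish velocity from the avatar's velocity.
; The ability ends when the force finishes, independent of montage completion.
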(event Ability|EventActivateAbility
  (bind _returnvalue (Ability|GetAvatarActorfromActorInfo))
  (bind _returnvalue_2 (Ability|GetAvatarActorfromActorInfo))
  (Ability|CommitAbility)
  (Variables|Default|SetPlayerForwardLocation (Transformation|GetActorForwardVector _returnvalue))
  (Class|CombatInterface|UpdateFacingTarget(Message) _returnvalue (Variables|Default|GetPlayerForwardLocation))
  (Niagara|SpawnSystematLocation (Variables|Default|GetDashNiagaraEffect) (Transformation|GetActorLocation _returnvalue_2) (Transformation|GetActorRotation _returnvalue_2) (Class|Actor|GetActorRelativeScale3D _returnvalue_2))
  (|PlayMontageandWaitProxy "None" (Variables|Default|GetMontage%20to%20Play) 1.0 "None" true 1.0 0.0 false
    (:then
      (Ability|Tasks|ApplyRootMotionConstantForce "None" (Variables|Default|GetPlayerForwardLocation) 7.5e+03 0.35 false 0 "SetVelocity" (Transformation|GetVelocity (Ability|GetAvatarActorfromActorInfo)) 1.0 true
        (:OnFinish
          (Ability|EndAbility))))))

(event Ability|EventOnEndAbility
  (params (bWasCancelled :type Boolean)))