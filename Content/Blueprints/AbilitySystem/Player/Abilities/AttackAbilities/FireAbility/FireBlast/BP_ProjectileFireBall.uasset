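; Fire blast fireball projectile that flies out along its forward vector, boomerangs back to its ReturnToActor, then explodes.
; On the authority, an outgoing timeline lerps it to the apex, then a returning timeline lerps it toward the actor's current location.
; Once within ExplodeDistance, it calls OnHit, applies radial damage with outward knockback and death impulse to nearby live players except its owner, and destroys itself.
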(event EventStartOutgoingTimeline
  (bind _returnvalue (Components|GetOwner))
  (bind _array (Utilities|Array|MakeArray _returnvalue))
  (Networking|SwitchHasAuthority
    (:Authority
      ;[0.6146 0.4457 0] Store Initial & Apex Locations
      (Variables|Default|SetInitialLocation (Transformation|GetActorLocation))
      (Variables|Default|SetApexLocation (+ (Variables|Default|GetInitialLocation) (* (Transformation|GetActorForwardVector) (Variables|Default|GetTravelDistance))))
      (bind _outgoingtrack (Timeline|OutgoingTimeline Play)
        (:Update
          (Transformation|SetActorLocation (Math|Vector|Lerp(Vector) (Variables|Default|GetInitialLocation) (Variables|Default|GetApexLocation) _outgoingtrack) false false))
        (:Finished
          (bind _returningtrack (Timeline|ReturningTimeline Play)
            (:Update
              (Transformation|SetActorLocation (Math|Vector|Lerp(Vector) (Variables|Default|GetApexLocation) (Transformation|GetActorLocation (Variables|Default|GetReturnToActor)) _returningtrack) false false)
              (if (CallFunction|IsWithinExplodeDistance)
                (Class|KDProjectile|OnHit)
                (Class|KDAbilitySystemLibrary|SetIsRadialDamageEffectParam (Variables|Default|GetExplosionDamageParams) true 5e+01 3e+02 (Transformation|GetActorLocation))
                (Utilities|Array|Add _array self)
                (bind _outoverlappingactors (Class|KDAbilitySystemLibrary|GetLivePlayersWithinRadius self _array 3e+02 (Transformation|GetActorLocation)))
                (for _array_element _outoverlappingactors
                  (Class|KDAbilitySystemLibrary|SetTargetEffectParamsASC (Variables|Default|GetExplosionDamageParams) (Ability|GetAbilitySystemComponent _array_element))
                  (Class|KDAbilitySystemLibrary|SetKnockbackDirectionDamageEffectParam (Variables|Default|GetExplosionDamageParams) (- (Transformation|GetActorLocation _array_element) (Transformation|GetActorLocation)) 2e+03)
                  (Class|KDAbilitySystemLibrary|SetDeathImpulseDirectionDamageEffectParam (Variables|Default|GetExplosionDamageParams) (- (Transformation|GetActorLocation _array_element) (Transformation|GetActorLocation)) 5e+02)
                  (Class|KDAbilitySystemLibrary|ApplyDamageEffect (Variables|Default|GetExplosionDamageParams)))
                (Actor|DestroyActor)))))))))

(fn ConstructionScript)

(fn IsWithinExplodeDistance
  (return (<= (Math|Vector|VectorLength (- (Transformation|GetActorLocation) (Transformation|GetActorLocation (Variables|Default|GetReturnToActor)))) (Variables|Default|GetExplodeDistance))))