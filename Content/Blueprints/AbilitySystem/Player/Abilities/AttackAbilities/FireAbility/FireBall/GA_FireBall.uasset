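; GA_FireBall is a player gameplay ability that casts fireball projectiles at whatever is under the mouse.
; On activation it commits, takes the hit location and actor from TargetDataUnderMouse, turns the avatar toward that point and plays the cast montage.
; The montage's gameplay event triggers SpawnProjectiles from the weapon socket with a pitch override, homing on the hit actor.
; The ability ends after spawning or when the montage finishes or breaks off.
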(event Ability|EventActivateAbility
  (Ability|CommitAbility)
  (bind _datahandle (|TargetDataUnderMouse)
    (:ValidData
      (Variables|Default|SetProjectileTargetLocation (.Location (Collision|BreakHitResult (Ability|TargetData|GetHitResultfromTargetData _datahandle))))
      (Variables|Default|SetMouseHit%20Actor (.HitActor (Collision|BreakHitResult (Ability|TargetData|GetHitResultfromTargetData _datahandle))))
      (Class|CombatInterface|UpdateFacingTarget(Message) (Ability|GetAvatarActorfromActorInfo) (Variables|Default|GetProjectileTargetLocation))
      (|PlayMontageandWaitProxy "None" (Variables|Default|GetMontageFireBall) 1.0 "None" true 1.0 0.0 false
        (:then
          (Ability|Tasks|WaitGameplayEvent "(TagName=\"Event.AnimMontage.FireBall\")" 0 true
            (:EventReceived
              (Class|KDFireBall|SpawnProjectiles (Variables|Default|GetProjectileTargetLocation) (GameplayTags|MakeLiteralGameplayTag "(TagName=\"CombatSocket.Weapon\")") true 25.0 (Variables|Default|GetMouseHit%20Actor))
              (Ability|EndAbility))))
        (:OnCompleted
          (Ability|EndAbility :!label _label))
        (:OnBlendOut
          (goto _label))
        (:OnInterrupted
          (goto _label))
        (:OnCancelled
          (goto _label))))))

(event Ability|EventOnEndAbility
  (params (bWasCancelled :type Boolean)))