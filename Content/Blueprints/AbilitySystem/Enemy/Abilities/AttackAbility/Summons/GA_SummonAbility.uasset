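; Enemy gameplay ability that summons random minions around the caster, using the Lich call montage.
; On activation it shuffles the spawn locations and plays a summon effect at every one.
; When the montage sends its attack gameplay event, a delay loop spawns one minion per location a second apart, raised slightly, facing away from the caster and given a default controller.
; The graph never calls EndAbility or resets the spawn index.
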(event Ability|EventActivateAbility
  (bind _returnvalue (Class|KDSummonAbility|GetSpawnLocation))
  (bind _output_get (Variables|Default|SetSpawnLocation _returnvalue))
  (Utilities|Array|Shuffle _output_get)
  (for _array_element (Variables|Default|GetSpawnLocation)
    (Niagara|SpawnSystematLocation (Variables|Default|GetSummon%20Effect) _array_element))
  (|PlayMontageandWaitProxy "None" "/Game/Blueprints/Characters/Enemy/Lich/AnimMontages/AM_Lich_Call.AM_Lich_Call" 1.0 "None" true 1.0 0.0 false
    (:then
      (Ability|Tasks|WaitGameplayEvent "(TagName=\"Montage.Attack.01\")" 0
        (:EventReceived
          (if (< (Variables|Default|GetSpawnLocationIndex) (Utilities|Array|Length (Variables|Default|GetSpawnLocation))) :!label _label
            (bind _returnvalue_2 (Game|SpawnActorfromClass (Class|KDSummonAbility|GetRandomMinionClass) (Math|Transform|MakeTransform (+ (Utilities|Array|Get(acopy) (Variables|Default|GetSpawnLocation) (Variables|Default|GetSpawnLocationIndex)) "0.000000,0.000000,70.000000") (Math|Rotator|FindLookatRotation (Transformation|GetActorLocation (Ability|GetAvatarActorfromActorInfo)) (+ (Utilities|Array|Get(acopy) (Variables|Default|GetSpawnLocation) (Variables|Default|GetSpawnLocationIndex)) "0.000000,0.000000,70.000000")) "1.000000,1.000000,1.000000") "AlwaysSpawn" "MultiplyWithRoot" 0 0))
            (Pawn|SpawnDefaultController _returnvalue_2)
            (Math|Integer|IncrementInt (Variables|Default|GetSpawnLocationIndex)
              (:%20%20
                (Utilities|FlowControl|Delay 1.0)
                (goto _label)))))))))

(event Ability|EventOnEndAbility
  (params (bWasCancelled :type Boolean)))