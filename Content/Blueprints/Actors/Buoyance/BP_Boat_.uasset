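; BP_Boat is a boat actor that slides along the world Y axis when play begins.
; BeginPlay stores its starting location, doubles that vector as the target, and calls the Floating event.
; Floating plays the Move timeline, which interpolates Y from start to target while setting X to a hardcoded value.
; Despite the Buoyance folder, it contains no buoyancy or physics logic.
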(event Custom|Floating
  (bind _move (Timeline|Move Play)
    (:Update
      (Transformation|SetActorLocation (Math|Vector|MakeVector -7.5e+03 (.y (Math|Vector|Lerp(Vector) (Variables|Default|GetLocation) (Variables|Default|GetNewLocation) _move)) 0.0) false false))))

(event EventBeginPlay
  (bind _output_get (Variables|Default|SetLocation (Transformation|GetActorLocation)))
  (Variables|Default|SetNewLocation (+ _output_get (Variables|Default|GetLocation)))
  (CallFunction|Floating))

(event Collision|EventActorBeginOverlap
  (params (OtherActor :type Actor%20Object%20Reference)))

(event EventTick
  (params (DeltaSeconds :type Float%20%28single-precision%29)))

(fn ConstructionScript)