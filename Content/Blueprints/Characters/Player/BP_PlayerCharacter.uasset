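; BP_PlayerCharacter is the player character Blueprint, handling dash input, interaction and camera-driven fading.
; It grants an ability through KDAbilitySystemComponent on BeginPlay, activates dash by tag on Spacebar, and feeds a FacingTarget location to Motion Warping.
; A camera box sends fade messages to overlapping BI_FadeInterface actors.
; Interact input and box exit message the stored Interactable, but overlap-begin is empty and its detection logic is disconnected.
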(event OnComponentBeginOverlap(BoxOverlap)
  (params (OverlappedComponent :type Primitive%20Component%20Object%20Reference) (OtherActor :type Actor%20Object%20Reference) (OtherComp :type Primitive%20Component%20Object%20Reference) (OtherBodyIndex :type Integer) (bFromSweep :type Boolean) (SweepResult :type Hit%20Result%20Structure%20%28by%20ref%29)))

(event OnComponentEndOverlap(BoxOverlap)
  (params (OverlappedComponent :type Primitive%20Component%20Object%20Reference) (OtherActor :type Actor%20Object%20Reference) (OtherComp :type Primitive%20Component%20Object%20Reference) (OtherBodyIndex :type Integer))
  (if (Utilities|DoesObjectImplementInterface OtherActor "/Game/TestingContent/BI_Interactable.BI_Interactable_C")
    (Utilities|IsValid (Variables|Default|GetInteractable)
      (:Is%20Valid
        (Class|BIInteractable|StopInteract(Message) (Variables|Default|GetInteractable))
        (Variables|Default|SetInteractable (Variables|Default|GetInteractable))))))

(event OnComponentBeginOverlap(CameraBoxComponent)
  (params (OverlappedComponent :type Primitive%20Component%20Object%20Reference) (OtherActor :type Actor%20Object%20Reference) (OtherComp :type Primitive%20Component%20Object%20Reference) (OtherBodyIndex :type Integer) (bFromSweep :type Boolean) (SweepResult :type Hit%20Result%20Structure%20%28by%20ref%29))
  (if (Utilities|DoesObjectImplementInterface OtherActor "/Game/Blueprints/Actors/FadeActor/BI_FadeInterface.BI_FadeInterface_C")
    (Class|BIFadeInterface|FadeOut(Message) OtherActor)))

(event OnComponentEndOverlap(CameraBoxComponent)
  (params (OverlappedComponent :type Primitive%20Component%20Object%20Reference) (OtherActor :type Actor%20Object%20Reference) (OtherComp :type Primitive%20Component%20Object%20Reference) (OtherBodyIndex :type Integer))
  (if (Utilities|DoesObjectImplementInterface OtherActor "/Game/Blueprints/Actors/FadeActor/BI_FadeInterface.BI_FadeInterface_C")
    (Class|BIFadeInterface|Fadein(Message) OtherActor)))

(event Input|EnhancedActionEvents|EnhancedInputActionIA_Spacebar
  (params (ActionValue :type Float%20%28double-precision%29) (ElapsedSeconds :type Float%20%28double-precision%29) (TriggeredSeconds :type Float%20%28double-precision%29) (InputAction :type Input%20Action%20Object%20Reference :default "/Game/Blueprints/Inputs/InputActions/IA_Spacebar.IA_Spacebar"))
  (:Started
    (Abilities|TryActivateAbilitiesbyTag (Variables|Default|GetKDAbility%20System%20Component) (Variables|Default|GetAbilityDash) true)))

(event Input|EnhancedActionEvents|EnhancedInputActionIA_Interact
  (params (ActionValue :type Boolean) (ElapsedSeconds :type Float%20%28double-precision%29) (TriggeredSeconds :type Float%20%28double-precision%29) (InputAction :type Input%20Action%20Object%20Reference :default "/Game/Blueprints/Inputs/InputActions/IA_Interact.IA_Interact"))
  (:Started
    (Utilities|IsValid (Variables|Default|GetInteractable)
      (:Is%20Valid
        (Class|BIInteractable|StartInteract(Message) (Variables|Default|GetInteractable))))))

(event EventBeginPlay
  (bind _askdability_system_component (Utilities|Casting|CastToKDAbilitySystemComponent (Ability|GetAbilitySystemComponent 0)))
  (Variables|Default|SetKDAbility%20System%20Component _askdability_system_component)
  (GameplayAbilities|GiveAbility (Variables|Default|GetKDAbility%20System%20Component) (Variables|Default|GetAbility%20Class) 0 -1))

(event EventUpdateFacingTarget
  (params (Target :type Vector%20%28by%20ref%29 :default "0, 0, 0"))
  (Class|MotionWarpingComponent|AddorUpdateWarpTargetfromLocation (Variables|Default|GetMotionWarping) "FacingTarget" Target))

(event EventSetinShockLoop
  (params (bInLoop :type Boolean))
  (Variables|Default|SetInShockLoop bInLoop))

(fn ConstructionScript)