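; Player controller that sets up the HUD's viewport widget and reports whether the player may move or look, based on dialogue state.
; On BeginPlay, where cosmetic events can run and the controller is local, it initializes the widget through the HUD and adds it to the player screen.
; CanMove and CanLook read the PlayerState's MounteaDialogueManager state, returning false while Active and true otherwise or without a valid PlayerState.
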(event EventBeginPlay
  (bind _returnvalue (HUD|GetHUD))
  (Networking|CanExecuteCosmeticEvents
    (:True
      (if (Pawn|IsLocalPlayerController)
        (Class|MounteaDialogueHUDStatics|InitializeViewportWidget _returnvalue)
        (UserInterface|Viewport|AddtoPlayerScreen (Class|MounteaDialogueHUDStatics|GetViewportWidget _returnvalue))))))

(event EventTick
  (params (DeltaSeconds :type Float%20%28single-precision%29)))

(fn ConstructionScript)

(fn CanMove
  (bind _playerstate (Variables|Default|GetPlayerState)
    (:then
      (return (Utilities|Select :Index (Class|MounteaDialogueManagerStatics|GetManagerState (Actor|GetComponentbyClass _playerstate "/Script/MounteaDialogueSystem.MounteaDialogueManager")) :EDMS_Disabled true :EDMS_Enabled true :EDMS_Active false)))
    (:else
      (return true))))

(fn CanLook
  (bind _playerstate (Variables|Default|GetPlayerState)
    (:then
      (return (Utilities|Select :Index (Class|MounteaDialogueManagerStatics|GetManagerState (Actor|GetComponentbyClass _playerstate "/Script/MounteaDialogueSystem.MounteaDialogueManager")) :EDMS_Disabled true :EDMS_Enabled true :EDMS_Active false)))
    (:else
      (return true))))