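; BP_NPC_Reas is an NPC that takes part in Mountea dialogues, giving visual feedback through its widget component and a dynamic mesh material.
; Participant state changes register the widget with the dialogue manager and tint the mesh black when Active after a short delay, or remove and reset them otherwise.
; Dialogue updates, briefly delayed, show the widget's row only when the active row matches this participant.
; All visual work is gated by a cosmetic-events check.
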(event OnDialogueParticipantStateChanged(NPC_MounteaDialogueParticipant)
  (params (NewState :type EDialogueParticipantState%20Enum%20%28by%20ref%29 :default "EDPS_Disabled"))
  (Networking|CanExecuteCosmeticEvents
    (:True
      (switch Utilities|FlowControl|Switch|SwitchonEDialogueParticipantState NewState
        (:EDPS_Disabled
          (Class|MounteaDialogueManagerStatics|RemoveDialogueUIObject (Class|MounteaDialogueParticipantStatics|GetDialogueManager (Variables|Default|GetNPC_MounteaDialogueParticipant)) (UserInterface|GetWidget (Variables|Default|GetWidget)) :!label _label)
          (bind _dynamicmaterial (Variables|Default|GetDynamicMaterial)
            (:then
              (Rendering|Material|SetVectorParameterValue _dynamicmaterial "Tint" "(R=1.000000,G=1.000000,B=1.000000,A=1.000000)" :!class /Script/Engine.MaterialInstanceDynamic))
            (:else)))
        (:EDPS_Enabled
          (goto _label))
        (:EDPS_Active
          (Utilities|FlowControl|Delay 1.0)
          (Class|MounteaDialogueManagerStatics|AddDialogueUIObject (Class|MounteaDialogueParticipantStatics|GetDialogueManager (Variables|Default|GetNPC_MounteaDialogueParticipant)) (UserInterface|GetWidget (Variables|Default|GetWidget)))
          (bind _dynamicmaterial_2 (Variables|Default|GetDynamicMaterial)
            (:then
              (Rendering|Material|SetVectorParameterValue :self _dynamicmaterial_2 :ParameterName "Tint" :!class /Script/Engine.MaterialInstanceDynamic))
            (:else)))))))

(event OnDialogueUpdated(NPC_MounteaDialogueParticipant)
  (params (OwningManager :type Mountea%20Dialogue%20Manager%20Interface%20Interface%20%28by%20ref%29))
  (Utilities|FlowControl|Delay 0.1)
  (CallFunction|ProcessDialogueUpdated OwningManager))

(event EventBeginPlay
  (|CallParentFunction)
  (Networking|CanExecuteCosmeticEvents
    (:True
      (Variables|Default|GetDynamicMaterial
        (:then)
        (:else
          (bind _returnvalue (Rendering|Material|CreateDynamicMaterialInstance (Variables|Character|GetMesh) 0 0 "None" :!class /Script/Engine.PrimitiveComponent))
          (Variables|Default|SetDynamicMaterial _returnvalue))))))

(event Collision|EventActorBeginOverlap
  (params (OtherActor :type Actor%20Object%20Reference)))

(event EventTick
  (params (DeltaSeconds :type Float%20%28single-precision%29)))

(fn ConstructionScript
  (|CallParentFunction))

(fn ProcessDialogueUpdated
  (params (Target :type Mountea%20Dialogue%20Manager%20Interface%20Interface))
  (bind _returnvalue (Class|MounteaDialogueManagerStatics|GetDialogueContext Target))
  (Networking|CanExecuteCosmeticEvents
    (:True
      (if (Class|MounteaDialogueSystemBFC|IsContextValid _returnvalue)
        (switch Utilities|FlowControl|Switch|SwitchonEDialogueParticipantState (Class|MounteaDialogueParticipantStatics|GetParticipantState (Variables|Default|GetNPC_MounteaDialogueParticipant))
          (:EDPS_Disabled
            (Class|MounteaDialogueHUDStatics|RefreshDialogueWidget (UserInterface|GetWidget (Variables|Default|GetWidget)) Target "HideRow" :!label _label))
          (:EDPS_Enabled
            (goto _label))
          (:EDPS_Active
            (Class|MounteaDialogueHUDStatics|RefreshDialogueWidget (UserInterface|GetWidget (Variables|Default|GetWidget)) Target (Utilities|String|SelectString "ShowRow" "HideRow" (Class|MounteaDialogueSystemBFC|DoesRowMatchParticipant (Variables|Default|GetNPC_MounteaDialogueParticipant) (Variables|/Script/MounteaDialogueSystem.MounteaDialogueContext|GetActiveDialogueRow _returnvalue))))))))))