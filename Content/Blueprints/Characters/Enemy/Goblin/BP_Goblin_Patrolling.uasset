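; Goblin enemy variant that wanders the level on its own, starting at BeginPlay after the parent's logic runs.
; MoveToRandomLocation picks a random navigable point within a fixed radius of the current position and sends the pawn there with AIMoveTo.
; Success calls the event again for an endless roam that drifts from the spawn point, while a failed move has no handler and ends the loop.
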(event Custom|MoveToRandomLocation
  (bind _randomlocation (Class|NavigationSystemV1|GetRandomLocationinNavigableRadius (Transformation|GetActorLocation) 5e+02 0 0))
  (AI|AIMoveTo self _randomlocation 0 5.0 false
    (:OnSuccess
      (CallFunction|MovetoRandomLocation))))

(event EventBeginPlay
  (|CallParentFunction)
  (CallFunction|MovetoRandomLocation))

(event Collision|EventActorBeginOverlap
  (params (OtherActor :type Actor%20Object%20Reference))
  (|CallParentFunction OtherActor) ; This node is disabled and will not be called.\nDrag off pins to build functionality.
)

(event EventTick
  (params (DeltaSeconds :type Float%20%28single-precision%29))
  (|CallParentFunction DeltaSeconds) ; This node is disabled and will not be called.\nDrag off pins to build functionality.
)

(fn ConstructionScript
  (|CallParentFunction))