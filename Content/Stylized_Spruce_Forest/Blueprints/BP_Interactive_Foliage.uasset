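; Interactive foliage Blueprint that feeds its own speed and position to materials through MPC_Global, for bending foliage around the moving actor.
; Each Tick it eases PlayerSpeed toward its tightly clamped velocity magnitude, so it acts mostly as a smoothed moving-or-still factor.
; PlayerPosition trails a point one unit behind the actor via VInterpTo, delaying the bend.
; Both values are written to the parameter collection; the bending itself happens outside this Blueprint.
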(event EventTick
  (params (DeltaSeconds :type Float%20%28single-precision%29))
  (bind _returnvalue (Utilities|Time|GetWorldDeltaSeconds))
  ;[1 1 1] InteractiveFoliage
  (bind _output_get (Variables|Components|SetPlayerSpeed (Math|Interpolation|FInterpTo (Variables|Components|GetPlayerSpeed) (Math|Float|Clamp(Float) (Math|Vector|VectorLength (Transformation|GetVelocity)) 0.0 0.01) _returnvalue 1.0)))
  (Rendering|Material|SetScalarParameterValue "/Game/Stylized_Spruce_Forest/MPC/MPC_Global.MPC_Global" "PlayerSpeed" _output_get :!class /Script/Engine.KismetMaterialLibrary)
  (Variables|Components|SetPlayer%20Position (Math|Interpolation|VInterpTo (Variables|Components|GetPlayer%20Position) (+ (Math|Vector|NegateVector (Transformation|GetActorForwardVector)) (Transformation|GetActorLocation)) _returnvalue 2.0))
  (Rendering|Material|SetVectorParameterValue "/Game/Stylized_Spruce_Forest/MPC/MPC_Global.MPC_Global" "Player Position" (Math|Conversions|ToLinearColor(Vector) (Math|Interpolation|VInterpTo (Variables|Components|GetPlayer%20Position) (+ (Math|Vector|NegateVector (Transformation|GetActorForwardVector)) (Transformation|GetActorLocation)) _returnvalue 2.0)) :!class /Script/Engine.KismetMaterialLibrary))

(event Collision|EventActorBeginOverlap
  (params (OtherActor :type Actor%20Object%20Reference)))

(fn ConstructionScript)