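; BP_Info is an interactable actor that pages through a text sequence in an on-screen information or dialogue widget.
; CanInteract shows its Widget prompt, while StopInteract hides it and clears any open display.
; StartInteract hides the prompt and creates the display class mapped to SelectedInteractionType, or advances the text if one is open.
; Advancing past the last entry removes the display and resets the index.
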(event EventBeginPlay)

(event Collision|EventActorBeginOverlap
  (params (OtherActor :type Actor%20Object%20Reference)))

(event EventStopInteract
  (bind _widget (Variables|Default|GetWidget)
    (:then
      (Rendering|SetVisibility _widget false false)
      (Variables|Default|GetDisplayedWidget
        (:then
          (CallFunction|ResetUI))
        (:else)))
    (:else)))

(event EventCanInteract
  (bind _widget (Variables|Default|GetWidget)
    (:then
      (Rendering|SetVisibility _widget true false))
    (:else)))

(event EventTick
  (params (DeltaSeconds :type Float%20%28single-precision%29)))

(event EventStartInteract
  (bind _widget (Variables|Default|GetWidget)
    (:then
      (Rendering|SetVisibility _widget false false)
      (Variables|Default|GetDisplayedWidget
        (:then
          (CallFunction|UpdateTexttoDisplay)
          (CallFunction|SetTexttoDisplay))
        (:else
          (CallFunction|AddWidgettoViewport)
          (CallFunction|SetTexttoDisplay))))
    (:else)))

(fn ConstructionScript)

(fn UpdateTexttoDisplay
  (if (< (Variables|Default|GetTextToDisplay) (- (Utilities|Array|Length (Variables|Default|GetTextSequence)) 1))
    (Math|Integer|IncrementInt (Variables|Default|GetTextToDisplay))
    (else
      (CallFunction|ResetUI))))

(fn ResetUI
  (Widget|RemovefromParent (Variables|Default|GetDisplayedWidget))
  (Variables|Default|SetDisplayedWidget 0)
  (Rendering|SetVisibility (Variables|Default|GetWidget) false false)
  (Variables|Default|SetTextToDisplay 0))

(fn SetTexttoDisplay
  (bind _aswbp_information_display (Utilities|Casting|CastToWBP_InformationDisplay (Variables|Default|GetDisplayedWidget))
    (:then
      (Variables|/Game/TestingContent/Widgets/WBP_InformationDisplay.WBP_InformationDisplay_C|SetTextToDisplay _aswbp_information_display (Utilities|Array|Get(acopy) (Variables|Default|GetTextSequence) (Variables|Default|GetTextToDisplay))))
    (:CastFailed
      (bind _aswbp_dialogue_display (Utilities|Casting|CastToWBP_DialogueDisplay (Variables|Default|GetDisplayedWidget)))
      (Variables|/Game/TestingContent/Widgets/WBP_DialogueDisplay.WBP_DialogueDisplay_C|SetTextToDisplay _aswbp_dialogue_display (Utilities|Array|Get(acopy) (Variables|Default|GetTextSequence) (Variables|Default|GetTextToDisplay))))))

(fn AddWidgettoViewport
  (bind _interactiontypemap (Variables|Default|GetInteractionTypeMap))
  (bind _selectedinteractiontype (Variables|Default|GetSelectedInteractionType))
  (bind (_value _returnvalue) (Utilities|Map|Find _interactiontypemap _selectedinteractiontype))
  (if _returnvalue
    (bind _output_get (Variables|Default|SetWidgetToDisplay _value))
    (bind _returnvalue_2 (UserInterface|CreateWidget _output_get))
    (Utilities|IsValid _returnvalue_2
      (:Is%20Valid
        (bind _output_get_2 (Variables|Default|SetDisplayedWidget _returnvalue_2))
        (UserInterface|Viewport|AddtoViewport _output_get_2 0)))))